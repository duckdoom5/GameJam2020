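; Player character for the bottom half of a team-coloured egg, with stick movement and aiming, that throws and recalls its separate top half.
; The Top actor's state drives the logic: holding Throw charges speed, release or timeout launches it via an added projectile component, and pressing again recalls it along a curve.
; Death splashes or, 10% of the time, flings the egg at the camera, then notifies the game mode and respawns it from above.
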(event Custom|AutoFire
  ;[1 1 1] Throw
  (if (Utilities|Enum|Equal(Enum) (Variables|/Game/Blueprints/Player/BP_EggTop.BP_EggTop_C|GetState (Variables|Default|Gettop)) "NewEnumerator5")
    (Variables|/Game/Blueprints/Player/BP_EggTop.BP_EggTop_C|SetState (Variables|Default|Gettop) "NewEnumerator6")
    (Utilities|FlowControl|Delay 0.5) ; Wait for anim
    (CallFunction|FireTop)))

(event Custom|PlayerDeath
  (bind _arrow1 (Variables|Default|GetArrow1))
  (bind _chargingrumble (Variables|Default|GetChargingRumble))
  (bind _top (Variables|Default|Gettop))
  (bind _returnvalue (Transformation|GetWorldScale _arrow1))
  ;[1 1 1] Death
  (if (not (or (Utilities|Enum|Equal(Enum) (Variables|/Game/Blueprints/Player/BP_EggTop.BP_EggTop_C|GetState _top) "NewEnumerator9") (Utilities|Enum|Equal(Enum) (Variables|/Game/Blueprints/Player/BP_EggTop.BP_EggTop_C|GetState _top) "NewEnumerator10")))
    (bind _asbp_game_mode (Utilities|Casting|CastToBP_GameMode (Game|GetGameMode)))
    (Camera|PlayWorldCameraShake "/Game/Blueprints/Player/HitShake.HitShake_C" (Transformation|GetWorldLocation (Variables|/Game/Blueprints/BP_Camera.BP_Camera_C|GetCamera (Variables|Default|GetCamera))) 1e+02 2e+02)
    (if (<= (Math|Random|RandomFloat) 0.1)
      (CallFunction|PrepFling)
      (else
        (Effects|SpawnEmitteratLocation "/Game/VFX/P_EggSplash.P_EggSplash" (Transformation|GetActorLocation) "0, 0, 0" (Math|Conversions|ToVector(Float) (Math|Random|RandomFloatinRange 0.8 1.2)))
        (Default|ResetTop (Variables|Default|Gettop))
        (Variables|Default|SetChargingTime 0.0)
        (Transformation|SetWorldScale3D _arrow1 (Math|Vector|MakeVector 0.5 (.y _returnvalue) (.z _returnvalue)))
        (Utilities|IsValid _chargingrumble
          (:Is%20Valid
            (Audio|Components|Audio|Stop _chargingrumble))
          (:Is%20Not%20Valid
            _))
        (Default|OnPlayerDeath _asbp_game_mode (Variables|Default|GetTeam))
        (Transformation|SetActorLocation "20000.000000, 0,-2000.000000" false true)
        (CallFunction|CombineEgg false)
        (Variables|/Game/Blueprints/Player/BP_EggTop.BP_EggTop_C|SetState (Variables|Default|Gettop) "NewEnumerator8")
        (Utilities|FlowControl|Delay 2.0)
        (CallFunction|Respawn)))))

(event Custom|Respawn
  (bind _spawnlocations (Variables|Default|GetSpawnLocations))
  ;[1 1 1] Respawn
  (Variables|/Game/Blueprints/Player/BP_EggTop.BP_EggTop_C|SetState (Variables|Default|Gettop) "NewEnumerator9")
  (Transformation|SetWorldLocation (Variables|Collision|GetCapsuleComponent) (+ (Transformation|GetActorLocation (Utilities|Array|Get(acopy) _spawnlocations (Math|Random|RandomIntegerinRange 0 (Utilities|Array|LastIndex _spawnlocations)))) "0, 0,1500.000000") false true))

(event Custom|UpdateState
  (bind _arrow1 (Variables|Default|GetArrow1))
  (bind _chargingrumble (Variables|Default|GetChargingRumble))
  (bind _returnvalue (Transformation|GetWorldScale _arrow1))
  ;[1 1 1] Update State
  (switch Utilities|FlowControl|Switch|SwitchonPlayerState (Variables|/Game/Blueprints/Player/BP_EggTop.BP_EggTop_C|GetState (Variables|Default|Gettop))
    (:NewEnumerator3
      (CallFunction|ReturntoPlayer))
    (:NewEnumerator5
      (CallFunction|Charge))
    (:NewEnumerator11
      (CallFunction|FlingPlayeratScreen)
      (Utilities|FlowControl|Delay 1.8)
      ;[1 1 1] Death
      (Default|ResetTop (Variables|Default|Gettop))
      (Variables|Default|SetChargingTime 0.0)
      (Transformation|SetWorldScale3D _arrow1 (Math|Vector|MakeVector 0.5 (.y _returnvalue) (.z _returnvalue)))
      (Utilities|IsValid _chargingrumble
        (:Is%20Valid
          (Audio|Components|Audio|Stop _chargingrumble))
        (:Is%20Not%20Valid
          _))
      (Default|OnPlayerDeath (stale Custom|PlayerDeath _asbp_game_mode) (Variables|Default|GetTeam))
      (Transformation|SetActorLocation "20000.000000, 0,-2000.000000" false true)
      (CallFunction|CombineEgg false)
      (Variables|/Game/Blueprints/Player/BP_EggTop.BP_EggTop_C|SetState (Variables|Default|Gettop) "NewEnumerator8")
      (Utilities|FlowControl|Delay 2.0)
      (CallFunction|Respawn))))

(event EventTick
  (params (DeltaSeconds :type Float%20%28single-precision%29))
  (Utilities|FlowControl|Sequence
    (:then_0
      ;[1 1 1] Smooth Rotation
      (Transformation|SetActorRotation (Math|Rotator|Lerp(Rotator) (Transformation|GetActorRotation) (Variables|Default|GetTargetRot) 0.1 true)))
    (:then_1
      (CallFunction|UpdateState))))

(event Collision|EventActorBeginOverlap
  (params (OtherActor :type Actor%20Object%20Reference)))

(event EventOnMovementModeChanged
  (params (PrevMovementMode :type EMovementMode%20Enum :default "MOVE_None") (NewMovementMode :type EMovementMode%20Enum :default "MOVE_None") (PrevCustomMode :type Byte :default 0) (NewCustomMode :type Byte :default 0))
  (if (and (Utilities|Enum|Equal(Enum) NewMovementMode "MOVE_Walking") (Utilities|Enum|Equal(Enum) (Variables|/Game/Blueprints/Player/BP_EggTop.BP_EggTop_C|GetState (Variables|Default|Gettop)) "NewEnumerator9"))
    (Variables|/Game/Blueprints/Player/BP_EggTop.BP_EggTop_C|SetState (Variables|Default|Gettop) "NewEnumerator10")
    (Utilities|FlowControl|Delay 1.0)
    (if (Utilities|Enum|Equal(Enum) (Variables|/Game/Blueprints/Player/BP_EggTop.BP_EggTop_C|GetState (Variables|Default|Gettop)) "NewEnumerator10") ; Make sure state is still landed after one second
      (Variables|/Game/Blueprints/Player/BP_EggTop.BP_EggTop_C|SetState (Variables|Default|Gettop) "NewEnumerator0"))))

(event EventBeginPlay
  ;[1 1 1] Player Color
  (Utilities|FlowControl|Sequence
    (:then_0
      (CallFunction|Respawn))
    (:then_1
      (bind _outactors (Actor|GetAllActorsOfClass "/Game/Blueprints/BP_Camera.BP_Camera_C"))
      (Variables|Default|SetCamera (Utilities|Array|Get(acopy) _outactors)))
    (:then_2
      (Variables|/Game/Blueprints/Player/BP_EggTop.BP_EggTop_C|SetEggOwner (Variables|Default|Gettop) self))))

(event Input|ActionEvents|InputActionThrow
  (params (Key :type Key%20Structure :default "None"))
  ;[1 1 1] Throw
  (:Pressed
    (switch Utilities|FlowControl|Switch|SwitchonPlayerState (Variables|/Game/Blueprints/Player/BP_EggTop.BP_EggTop_C|GetState (Variables|Default|Gettop))
      (:NewEnumerator0
        (Variables|/Game/Blueprints/Player/BP_EggTop.BP_EggTop_C|SetState (Variables|Default|Gettop) "NewEnumerator5")
        (bind _returnvalue (ForceFeedback|SpawnForceFeedbackAttached "/Game/Blueprints/Player/ChargingRumble.ChargingRumble" (Variables|Collision|GetCapsuleComponent) "None" "0, 0, 0" "0, 0, 0" "KeepRelativeOffset" false false 1.0 0.0 (Variables|Default|GetHapticRadius)))
        (Variables|Default|SetChargingRumble _returnvalue))
      (:NewEnumerator2
        (Collision|SetCollisionResponsetoChannel (Variables|/Game/Blueprints/Player/BP_EggTop.BP_EggTop_C|GetRoot (Variables|Default|Gettop)) "ECC_WorldStatic" "ECR_Ignore")
        (Variables|/Game/Blueprints/Player/BP_EggTop.BP_EggTop_C|SetState (Variables|Default|Gettop) "NewEnumerator3")
        (Variables|Default|SetInitialDistance (Math|Vector|Distance(Vector) (Transformation|GetWorldLocation (Variables|Default|GetAttachTop)) (Transformation|GetWorldLocation (Variables|/Script/Engine.Actor|GetRootComponent (Variables|Default|Gettop))))))))
  (:Released
    (if (Utilities|Enum|Equal(Enum) (Variables|/Game/Blueprints/Player/BP_EggTop.BP_EggTop_C|GetState (Variables|Default|Gettop)) "NewEnumerator5")
      (Variables|/Game/Blueprints/Player/BP_EggTop.BP_EggTop_C|SetState (Variables|Default|Gettop) "NewEnumerator6")
      (Utilities|FlowControl|Delay 0.5) ; Wait for anim
      (CallFunction|FireTop))))

(event Input|AxisEvents|InputAxisMoveForward
  (params (AxisValue :type Float%20%28single-precision%29))
  (bind _top (Variables|Default|Gettop))
  (bind _state (Variables|/Game/Blueprints/Player/BP_EggTop.BP_EggTop_C|GetState _top))
  ;[1 1 1] Movement
  (if (> (+ (Math|Float|Absolute(Float) AxisValue) (Math|Float|Absolute(Float) (stale Input|AxisEvents|InputAxisMoveRight AxisValue))) 0.2) ; Dead signal
    (if (not (or (Utilities|Enum|Equal(Enum) _state "NewEnumerator5") (Utilities|Enum|Equal(Enum) _state "NewEnumerator6"))) ; Slow down movement when throwing
      (Pawn|Input|AddMovementInput (Math|Vector|MakeVector AxisValue (stale Input|AxisEvents|InputAxisMoveRight AxisValue) 0.0) 1.0 false)
      (else
        (Pawn|Input|AddMovementInput (Math|Vector|MakeVector AxisValue (stale Input|AxisEvents|InputAxisMoveRight AxisValue) 0.0) 0.25 false)))
    (Variables|Default|SetMoveDir (Math|Vector|MakeVector AxisValue (stale Input|AxisEvents|InputAxisMoveRight AxisValue) 0.0))))

(event Input|AxisEvents|InputAxisMoveRight
  (params (AxisValue :type Float%20%28single-precision%29))
  (bind _top (Variables|Default|Gettop))
  (bind _state (Variables|/Game/Blueprints/Player/BP_EggTop.BP_EggTop_C|GetState _top))
  ;[1 1 1] Movement
  (if (> (+ (Math|Float|Absolute(Float) (stale Input|AxisEvents|InputAxisMoveForward AxisValue)) (Math|Float|Absolute(Float) AxisValue)) 0.2) ; Dead signal
    (if (not (or (Utilities|Enum|Equal(Enum) _state "NewEnumerator5") (Utilities|Enum|Equal(Enum) _state "NewEnumerator6"))) ; Slow down movement when throwing
      (Pawn|Input|AddMovementInput (Math|Vector|MakeVector (stale Input|AxisEvents|InputAxisMoveForward AxisValue) AxisValue 0.0) 1.0 false)
      (else
        (Pawn|Input|AddMovementInput (Math|Vector|MakeVector (stale Input|AxisEvents|InputAxisMoveForward AxisValue) AxisValue 0.0) 0.25 false)))
    (Variables|Default|SetMoveDir (Math|Vector|MakeVector (stale Input|AxisEvents|InputAxisMoveForward AxisValue) AxisValue 0.0))))

(event Input|AxisEvents|InputAxisAimForward
  (params (AxisValue :type Float%20%28single-precision%29))
  ;[1 1 1] Aiming
  (if (> (+ (Math|Float|Absolute(Float) AxisValue) (Math|Float|Absolute(Float) (stale Input|AxisEvents|InputAxisAimRight AxisValue))) 0.2)
    (Variables|Default|SetTargetRot (Math|Rotator|MakeRotator 0.0 0.0 (Class|KismetMathLibrary|DegAtan2 (stale Input|AxisEvents|InputAxisAimRight AxisValue) AxisValue)))))

(event Input|AxisEvents|InputAxisAimRight
  (params (AxisValue :type Float%20%28single-precision%29))
  ;[1 1 1] Aiming
  (if (> (+ (Math|Float|Absolute(Float) (stale Input|AxisEvents|InputAxisAimForward AxisValue)) (Math|Float|Absolute(Float) AxisValue)) 0.2)
    (Variables|Default|SetTargetRot (Math|Rotator|MakeRotator 0.0 0.0 (Class|KismetMathLibrary|DegAtan2 AxisValue (stale Input|AxisEvents|InputAxisAimForward AxisValue))))))

(fn ConstructionScript
  (CallFunction|CombineEgg false)
  (Variables|Default|SetSpawnPos (Transformation|GetActorLocation))
  (switch Utilities|FlowControl|Switch|SwitchonTeamEnum (Variables|Default|GetTeam)
    (:NewEnumerator0
      (Rendering|Material|SetMaterial (Variables|Character|GetMesh) 0 "/Game/Materials/Egg1_Btm_MI.Egg1_Btm_MI")
      (Rendering|Material|SetMaterial (Variables|/Game/Blueprints/Player/BP_EggTop.BP_EggTop_C|GetSkeletalMesh (Variables|Default|Gettop)) 0 "/Game/Materials/Egg1_Top_MI.Egg1_Top_MI"))
    (:NewEnumerator1
      (Rendering|Material|SetMaterial (Variables|Character|GetMesh) 0 "/Game/Materials/Egg2_Btm_MI.Egg2_Btm_MI")
      (Rendering|Material|SetMaterial (Variables|/Game/Blueprints/Player/BP_EggTop.BP_EggTop_C|GetSkeletalMesh (Variables|Default|Gettop)) 0 "/Game/Materials/Egg2_Top_MI.Egg2_Top_MI"))))

(fn CombineEgg
  (params (Shake? :type Boolean))
  (bind _top (Variables|Default|Gettop))
  (bind _top_2 (Variables|Default|Gettop))
  (bind _top_3 (Variables|Default|Gettop))
  (bind _attachtop (Variables|Default|GetAttachTop))
  (bind _projectile (Variables|/Game/Blueprints/Player/BP_EggTop.BP_EggTop_C|GetProjectile _top_2))
  (Utilities|IsValid _projectile
    (:Is%20Valid
      (Components|DestroyComponent _projectile))
    (:Is%20Not%20Valid
      _))
  (Utilities|IsValid _top
    (:Is%20Valid
      (Transformation|SetActorLocation _top (Transformation|GetWorldLocation _attachtop) false true)
      (Transformation|SetActorRotation _top (Transformation|GetWorldRotation _attachtop))
      (Transformation|AttachActorToActor _top_3 self "None" "KeepWorld" "KeepWorld" "KeepWorld" true)
      (Collision|SetActorEnableCollision _top_3 false)
      (Collision|SetCollisionResponsetoChannel (Variables|/Game/Blueprints/Player/BP_EggTop.BP_EggTop_C|GetRoot (Variables|Default|Gettop)) "ECC_WorldStatic" "ECR_Block")
      (Variables|/Game/Blueprints/Player/BP_EggTop.BP_EggTop_C|SetState (Variables|Default|Gettop) "NewEnumerator0")
      (if Shake?
        (ForceFeedback|SpawnForceFeedbackAttached "/Game/Blueprints/Player/RePairRumble.RePairRumble" (Variables|Collision|GetCapsuleComponent) "None" "0, 0, 0" "0, 0, 0" "KeepRelativeOffset" false false 1.0 0.0 (Variables|Default|GetHapticRadius))
        (Audio|SpawnSound2D "/Game/Sound/Cues/egg-suck-pop_Cue.egg-suck-pop_Cue" 1.5 1.0 0.0 0)))))

(fn ReturntoPlayer
  (bind _top (Variables|Default|Gettop))
  (bind _attachtop (Variables|Default|GetAttachTop))
  (bind _returnvalue (Transformation|GetWorldLocation _attachtop))
  (bind _rootcomponent (Variables|/Script/Engine.Actor|GetRootComponent _top))
  (bind _returnvalue_2 (Transformation|GetWorldLocation _rootcomponent))
  (bind _returnvalue_3 (- _returnvalue _returnvalue_2))
  (bind _returnvalue_4 (Math|Vector|VectorLength _returnvalue_3))
  (if (or (<= _returnvalue_4 (Variables|Default|GetPickupRadius)) (<= _returnvalue_4 (* (Utilities|Time|GetWorldDeltaSeconds) (Variables|Default|GetReturnSpeed))))
    (CallFunction|CombineEgg true)
    (else
      (Transformation|AddActorWorldOffset (Variables|Default|Gettop) (* (Math|Vector|Normalize _returnvalue_3) (* (Utilities|Time|GetWorldDeltaSeconds) (* (Math|Curves|GetFloatValue (Variables|Default|GetVelocityCurve) (Math|Float|NormalizetoRange (Math|Vector|VectorLength (- (Transformation|GetWorldLocation (Variables|Default|GetAttachTop)) (Transformation|GetWorldLocation (Variables|/Script/Engine.Actor|GetRootComponent (Variables|Default|Gettop))))) 0.0 (Variables|Default|GetInitialDistance))) (Variables|Default|GetReturnSpeed)))) true))))

(fn Charge
  (bind _max_charging_time (Variables|Default|GetMax%20Charging%20Time))
  (bind _output_get (Variables|Default|SetChargingTime (+ (Variables|Default|GetChargingTime) (Utilities|Time|GetWorldDeltaSeconds))))
  (Transformation|SetRelativeScale3D (Variables|Default|GetArrow1) (Math|Vector|MakeVector (Math|Float|MapRangeClamped _output_get 0.0 _max_charging_time 0.5 3.0) 1.0 1.0))
  (if (> _output_get _max_charging_time)
    (CallFunction|AutoFire)))

(fn FireTop
  (bind _chargingrumble (Variables|Default|GetChargingRumble))
  (bind _top (Variables|Default|Gettop))
  (if (Utilities|Enum|Equal(Enum) (Variables|/Game/Blueprints/Player/BP_EggTop.BP_EggTop_C|GetState (Variables|Default|Gettop)) "NewEnumerator6")
    (Collision|SetActorEnableCollision (Variables|Default|Gettop) true)
    (Collision|IgnoreActorwhenMoving (Variables|/Game/Blueprints/Player/BP_EggTop.BP_EggTop_C|GetRoot (Variables|Default|Gettop)) self true)
    (Transformation|DetachFromActor (Variables|Default|Gettop) "KeepWorld" "KeepWorld" "KeepWorld")
    (bind _returnvalue (AddComponent|AddProjectileMovementComponent _top))
    (bind _output_get (Variables|/Game/Blueprints/Player/BP_EggTop.BP_EggTop_C|SetProjectile _top _returnvalue))
    (Variables|/Script/Engine.ProjectileMovementComponent|SetMaxSpeed (Variables|/Game/Blueprints/Player/BP_EggTop.BP_EggTop_C|GetProjectile (Variables|Default|Gettop)) (Math|Float|MapRangeClamped (Variables|Default|GetChargingTime) 0.0 (Variables|Default|GetMax%20Charging%20Time) 1.5e+03 4e+03))
    (Variables|/Script/Engine.MovementComponent|SetVelocity _output_get (* (- (Transformation|GetActorForwardVector) "0.0,0.0,0.050000") (Class|MovementComponent|GetMaxSpeed (Variables|/Game/Blueprints/Player/BP_EggTop.BP_EggTop_C|GetProjectile (Variables|Default|Gettop)))))
    (Variables|/Game/Blueprints/Player/BP_EggTop.BP_EggTop_C|SetState (Variables|Default|Gettop) "NewEnumerator1")
    (Variables|Default|SetChargingTime 0.0)
    (Utilities|IsValid _chargingrumble
      (:Is%20Valid
        (Audio|Components|Audio|Stop _chargingrumble))
      (:Is%20Not%20Valid
        _))
    (Transformation|SetRelativeScale3D (Variables|Default|GetArrow1) (Math|Vector|MakeVector 0.5 1.0 1.0))))

(fn FlingPlayeratScreen
  (bind _output_get (Variables|Default|SetFlingAlpha (+ (Variables|Default|GetFlingAlpha) (Utilities|Time|GetWorldDeltaSeconds))))
  (Physics|AddImpulse (Variables|Character|GetCharacterMovement) (* (* (Math|Curves|GetVectorValue (Variables|Default|GetFlingCurve) _output_get) (Math|Vector|Normalize (- (Variables|Default|GetFlingEnd) (Variables|Default|GetFlingStart)))) 1.3e+02) true))

(fn PrepFling
  (Variables|/Game/Blueprints/Player/BP_EggTop.BP_EggTop_C|SetState (Variables|Default|Gettop) "NewEnumerator11")
  (Variables|Default|SetFlingAlpha 0.0)
  (Variables|Default|SetFlingStart (Transformation|GetActorLocation))
  (Variables|Default|SetFlingEnd (Transformation|GetWorldLocation (Variables|/Game/Blueprints/BP_Camera.BP_Camera_C|GetCamera (Variables|Default|GetCamera)))))