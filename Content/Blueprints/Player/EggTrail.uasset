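; EggTrail is an actor that draws a trail along the ground tracking an EggTop, from the trail's spawn point.
; While the egg is in one specific state, each Tick traces down to static world geometry, ignoring the egg's owner, and moves the actor to the hit.
; The trail component is rotated toward the saved start and X-scaled to span the distance.
; In other states, a timeline runs before destruction, with the fade still a TODO.
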(event EventBeginPlay
  (Variables|Default|SetStartLoc (Transformation|GetActorLocation)))

(event EventTick
  (params (DeltaSeconds :type Float%20%28single-precision%29))
  (bind _eggtop (Variables|Default|GetEggTop))
  (bind _eggtrail (Variables|Default|GetEggTrail))
  (bind _eggtop_2 (Variables|Default|GetEggTop))
  (bind _returnvalue (Transformation|GetWorldScale _eggtrail))
  (bind _returnvalue_2 (Transformation|GetActorLocation _eggtop_2))
  (Utilities|IsValid _eggtop
    (:Is%20Valid
      (if (Utilities|Enum|Equal(Enum) (Variables|/Game/Blueprints/Player/BP_EggTop.BP_EggTop_C|GetState _eggtop) "NewEnumerator1")
        (bind (_outhit _returnvalue_3) (Collision|LineTraceForObjects _returnvalue_2 (+ _returnvalue_2 "0, 0,-500.000000") (Utilities|Array|MakeArray "ObjectTypeQuery1") false (Utilities|Array|MakeArray (Variables|/Game/Blueprints/Player/BP_EggTop.BP_EggTop_C|GetEggOwner (Variables|Default|GetEggTop))) "None"))
        (if _returnvalue_3
          (Transformation|SetActorLocation (+ (.Location (Collision|BreakHitResult _outhit)) "0, 0,10.000000") false true)
          (Transformation|SetWorldRotation (Variables|Default|GetEggTrail) (Math|Rotator|MakeRotationfromAxes (Math|Vector|Normalize (- (Variables|Default|GetStartLoc) (+ (.Location (Collision|BreakHitResult _outhit)) "0, 0,10.000000"))) (Math|Vector|CrossProduct (Math|Vector|Normalize (- (Variables|Default|GetStartLoc) (+ (.Location (Collision|BreakHitResult _outhit)) "0, 0,10.000000"))) "0, 0,-1.000000") "0, 0,1.000000") false false)
          (Transformation|SetWorldScale3D (Variables|Default|GetEggTrail) (Math|Vector|MakeVector (/ (Math|Vector|VectorLength (- (Variables|Default|GetStartLoc) (+ (.Location (Collision|BreakHitResult _outhit)) "0, 0,10.000000"))) 4e+02) (.y _returnvalue) (.z _returnvalue))))
        (else
          (Timeline|FadeOut Play
            (:Finished
              (Actor|DestroyActor) ; TODO: Add fade out
            )))))))

(fn ConstructionScript)