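; BP_Player is a player character that moves, jumps, and colors its sphere green or blue for controller ID 0 or 1.
; Forward and right axes share one world-space movement input call.
; Releasing jump or moving downward switches to the multiplied gravity scale for a snappier fall, and any movement mode change restores standard gravity.
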(event Collision|EventActorBeginOverlap
  (params (OtherActor :type Actor%20Object%20Reference)))

(event EventTick
  (params (DeltaSeconds :type Float%20%28single-precision%29))
  (if (< (.z (Transformation|GetVelocity)) 0.0)
    (Variables|/Script/Engine.CharacterMovementComponent|SetGravityScale (Variables|Character|GetCharacterMovement) (Variables|Default|GetGravityScaleMultiplied))))

(event EventOnMovementModeChanged
  (params (PrevMovementMode :type EMovementMode%20Enum :default "MOVE_None") (NewMovementMode :type EMovementMode%20Enum :default "MOVE_None") (PrevCustomMode :type Byte :default 0) (NewCustomMode :type Byte :default 0))
  (Variables|/Script/Engine.CharacterMovementComponent|SetGravityScale (Variables|Character|GetCharacterMovement) (Variables|Default|GetStandardGravityScale)))

(event EventBeginPlay
  (bind _sphere (Variables|Default|GetSphere))
  (bind _asplayer_controller (Utilities|Casting|CastToPlayerController (Pawn|GetController)))
  (switch int (Class|GameplayStatics|GetPlayerControllerID _asplayer_controller)
    (:0
      (Rendering|Material|SetMaterial _sphere 0 "/Game/M_Green.M_Green"))
    (:1
      (Rendering|Material|SetMaterial _sphere 0 "/Game/M_Blue.M_Blue"))))

(event Input|ActionEvents|InputActionjump
  (params (Key :type Key%20Structure :default "None"))
  (:Pressed
    (Character|Jump))
  (:Released
    (Variables|/Script/Engine.CharacterMovementComponent|SetGravityScale (Variables|Character|GetCharacterMovement) (Variables|Default|GetGravityScaleMultiplied))))

(event Input|AxisEvents|InputAxisMoveForward
  (params (AxisValue :type Float%20%28single-precision%29))
  (Pawn|Input|AddMovementInput (Math|Vector|MakeVector AxisValue (stale Input|AxisEvents|InputAxisMoveRight AxisValue) 0.0) 1.0 false))

(event Input|AxisEvents|InputAxisMoveRight
  (params (AxisValue :type Float%20%28single-precision%29))
  (Pawn|Input|AddMovementInput (Math|Vector|MakeVector (stale Input|AxisEvents|InputAxisMoveForward AxisValue) AxisValue 0.0) 1.0 false))

(fn ConstructionScript)