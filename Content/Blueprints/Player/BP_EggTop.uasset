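; BP_EggTop is the player's thrown egg top, which damages other players' BP_EggBottom on overlap while flying or returning.
; A state-driven Tick spawns one EggTrail per throw at a downward-traced ground point, falling back to the actor's location.
; A hit in flight switches the Cone to physics tumbling with a velocity-signed angular impulse, and a timer then settles it to OnFloor.
; Returning disables physics and zeroes the Cone's rotation.
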(event OnComponentHit(Cone)
  (params (HitComponent :type Primitive%20Component%20Object%20Reference) (OtherActor :type Actor%20Object%20Reference) (OtherComp :type Primitive%20Component%20Object%20Reference) (NormalImpulse :type Vector :default "0, 0, 0") (Hit :type Hit%20Result%20Structure%20%28by%20ref%29))
  (bind _tumbleforce (Variables|Default|GetTumbleForce))
  (switch Utilities|FlowControl|Switch|SwitchonPlayerState (Variables|Default|GetState)
    (:NewEnumerator1
      (Utilities|Casting|CastToBP_EggBottom OtherActor
        (:then
          _)
        (:CastFailed
          _))
      (Variables|Default|SetState "NewEnumerator4")
      (Physics|SetSimulatePhysics (Variables|Default|GetCone) true)
      (bind _returnvalue (Physics|GetPhysicsLinearVelocity (Variables|Default|GetCone) "None"))
      (Class|PrimitiveComponent|AddAngularImpulseinRadians (Variables|Default|GetCone) (Math|Vector|MakeVector (* (Math|Float|Sign(Float) (.x _returnvalue)) _tumbleforce) (* (Math|Float|Sign(Float) (.y _returnvalue)) _tumbleforce) 0.0) "None" true)
      (Variables|Default|SetTumbleTimer (Variables|Default|GetTumbleDuration)))))

(event OnComponentBeginOverlap(Cone)
  (params (OverlappedComponent :type Primitive%20Component%20Object%20Reference) (OtherActor :type Actor%20Object%20Reference) (OtherComp :type Primitive%20Component%20Object%20Reference) (OtherBodyIndex :type Integer) (bFromSweep :type Boolean) (SweepResult :type Hit%20Result%20Structure%20%28by%20ref%29))
  (if (!= OtherActor (Variables|Default|GetEggOwner))
    (Utilities|Casting|CastToBP_EggBottom OtherActor)
    (switch Utilities|FlowControl|Switch|SwitchonPlayerState (Variables|Default|GetState)
      (:NewEnumerator1
        (Game|Damage|ApplyDamage 0 0.0 0 0)
        (Variables|Default|SetState "NewEnumerator4")
        (Components|DestroyComponent (Variables|Default|GetProjectile)))
      (:NewEnumerator3
        (Game|Damage|ApplyDamage 0 0.0 0 0)))))

(event EventTick
  (params (DeltaSeconds :type Float%20%28single-precision%29))
  (bind _returnvalue (Transformation|GetActorLocation))
  (switch Utilities|FlowControl|Switch|SwitchonPlayerState (Variables|Default|GetState)
    (:NewEnumerator1
      (goto _label Reset))
    (:NewEnumerator3
      (Physics|SetSimulatePhysics (Variables|Default|GetCone) false)
      (Transformation|SetWorldRotation (Variables|Default|GetCone) "0, 0, 0" false false))
    (:NewEnumerator4
      (bind _output_get (Variables|Default|SetTumbleTimer (- (Variables|Default|GetTumbleTimer) DeltaSeconds)))
      (if (<= _output_get 0.0)
        (Variables|Default|SetState "NewEnumerator2")))
    (:NewEnumerator6
      ;[1 1 1] Spawn egg trail
      (Utilities|FlowControl|DoOnce false :!label _label
        (:Completed
          (bind (_outhit _returnvalue_2) (Collision|LineTraceForObjects _returnvalue (+ _returnvalue "0, 0,-500.000000") (Utilities|Array|MakeArray "ObjectTypeQuery1") false 0 "None"))
          (if _returnvalue_2
            (bind _returnvalue_3 (Game|SpawnActorfromClass "/Game/Blueprints/Player/EggTrail.EggTrail_C" (Math|Transform|MakeTransform (+ (.Location (Collision|BreakHitResult _outhit)) "0, 0,10.000000") "0, 0, 0" "0.000000,1,1") "AdjustIfPossibleButAlwaysSpawn" 0 (Variables|Default|GetEggOwner)))
            (Variables|/Game/Blueprints/Player/EggTrail.EggTrail_C|SetEggTop _returnvalue_3 self)
            (else
              (bind _returnvalue_4 (Game|SpawnActorfromClass "/Game/Blueprints/Player/EggTrail.EggTrail_C" (Math|Transform|MakeTransform _returnvalue "0, 0, 0" "0.000000,1,1") "AdjustIfPossibleButAlwaysSpawn" 0 (Variables|Default|GetEggOwner)))
              (Variables|/Game/Blueprints/Player/EggTrail.EggTrail_C|SetEggTop _returnvalue_4 self))))))))

(event EventBeginPlay
  (Variables|Default|SetInitialConeRotation (Variables|/Script/Engine.SceneComponent|GetRelativeRotation (Variables|Default|GetCone))))

(fn ConstructionScript)