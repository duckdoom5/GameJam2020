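; Game mode for a two-team match, Yolkers versus Eggheads, that tracks each team's shared lives.
; On BeginPlay it sets the first player's view to the last BP_Camera actor found in the level.
; Each player death decrements that team's lives; at zero the opposing team wins, which currently only prints a message.
; GetTeamLives exposes the remaining count for a given team.
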(event Custom|OnPlayerDeath
  (params (Team :type TeamEnum%20Enum :default "NewEnumerator0"))
  (switch Utilities|FlowControl|Switch|SwitchonTeamEnum Team
    (:NewEnumerator0
      (bind _result (Math|Integer|DecrementInt (Variables|Default|GetLivesYolkers))
        (:%20%20
          (if (<= _result 0)
            (CallFunction|TeamWin "NewEnumerator1")))))
    (:NewEnumerator1
      (bind _result_2 (Math|Integer|DecrementInt (Variables|Default|GetLivesEggheads))
        (:%20%20
          (if (<= _result_2 0)
            (CallFunction|TeamWin "NewEnumerator0")))))))

(event Custom|TeamWin
  (params (WinningTeam :type TeamEnum%20Enum :default "NewEnumerator0"))
  (Development|PrintString (Utilities|String|Append (Utilities|String|EnumtoString WinningTeam) " win!")))

(event EventBeginPlay
  (Utilities|FlowControl|Sequence
    (:then_0
      (bind _outactors (Actor|GetAllActorsOfClass "/Game/Blueprints/BP_Camera.BP_Camera_C"))
      (Game|Player|SetViewTargetwithBlend (Game|GetPlayerController 0) (Utilities|Array|Get(acopy) _outactors (Utilities|Array|LastIndex _outactors)) 0.0 "VTBlend_Linear" 0.0 false))))

(fn ConstructionScript)

(fn GetTeamLives
  (params (Team :type TeamEnum%20Enum :default "NewEnumerator0"))
  (switch Utilities|FlowControl|Switch|SwitchonTeamEnum Team
    (:NewEnumerator0
      (return (Variables|Default|GetLivesYolkers)))
    (:NewEnumerator1
      (return (Variables|Default|GetLivesEggheads)))))