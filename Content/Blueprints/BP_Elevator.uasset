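; Counterweight elevator with two physics platforms, where bodies resting on one side lift the other.
; Overlap events track each platform's occupants, and every Tick their mass drives an upward force on the opposite platform, applied as an acceleration change.
; A downward trace at BeginPlay measures the floor distance, and each Tick both platforms' world Z is clamped to that distance above or below the root's starting height.
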(event Custom|OnActorBeginOverlap_Event_0
  (params (OverlappedActor :type Actor%20Object%20Reference) (OtherActor :type Actor%20Object%20Reference))
  (bind _asprimitive_component (Utilities|Casting|CastToPrimitiveComponent (Variables|/Script/Engine.Actor|GetRootComponent OtherActor)))
  (Utilities|Array|Add (Variables|Default|GetLeftOverlappingActors) _asprimitive_component))

(event Custom|OnActorEndOverlap_Event_0
  (params (OverlappedActor :type Actor%20Object%20Reference) (OtherActor :type Actor%20Object%20Reference))
  (bind _asprimitive_component (Utilities|Casting|CastToPrimitiveComponent (Variables|/Script/Engine.Actor|GetRootComponent OtherActor)))
  (Utilities|Array|RemoveItem (Variables|Default|GetLeftOverlappingActors) _asprimitive_component))

(event Custom|OnActorBeginOverlap_Event_1
  (params (OverlappedActor :type Actor%20Object%20Reference) (OtherActor :type Actor%20Object%20Reference))
  (bind _asprimitive_component (Utilities|Casting|CastToPrimitiveComponent (Variables|/Script/Engine.Actor|GetRootComponent OtherActor)))
  (Utilities|Array|Add (Variables|Default|GetRightOverlappingActors) _asprimitive_component))

(event Custom|OnActorEndOverlap_Event_1
  (params (OverlappedActor :type Actor%20Object%20Reference) (OtherActor :type Actor%20Object%20Reference))
  (bind _asprimitive_component (Utilities|Casting|CastToPrimitiveComponent (Variables|/Script/Engine.Actor|GetRootComponent OtherActor)))
  (Utilities|Array|RemoveItem (Variables|Default|GetRightOverlappingActors) _asprimitive_component))

(event EventBeginPlay
  (bind _defaultsceneroot (Variables|Default|GetDefaultSceneRoot))
  (bind _returnvalue (Transformation|GetWorldLocation _defaultsceneroot))
  (Utilities|FlowControl|Sequence
    (:then_0
      (bind _asprimitive_component (Utilities|Casting|CastToPrimitiveComponent (Variables|/Script/Engine.Actor|GetRootComponent (Variables|Default|GetLeftPlatform))))
      (Variables|Default|SetLeftPhysicsActor _asprimitive_component))
    (:then_1
      (bind _asprimitive_component_2 (Utilities|Casting|CastToPrimitiveComponent (Variables|/Script/Engine.Actor|GetRootComponent (Variables|Default|GetRightPlatform))))
      (Variables|Default|SetRightPhysicsActor _asprimitive_component_2))
    (:then_2
      (bind (_outhit _returnvalue_2) (Collision|LineTraceByChannel _returnvalue (+ _returnvalue "0, 0,-9999999.000000") "TraceTypeQuery1" false 0 "ForOneFrame"))
      (if _returnvalue_2
        (Variables|Default|SetDistanceToFloor (- (.distance _outhit) (.z (Variables|/Script/Engine.SceneComponent|GetRelativeLocation (Variables|Default|GetLeftPhysicsActor)))))
        (Variables|Default|SetInitialWorldZ (.z (.tracestart _outhit)))))
    (:then_3
      (EventDispatchers|AssignOnActorBeginOverlap (Variables|Default|GetLeftPlatform) (delegate Custom|OnActorBeginOverlap_Event_0))
      (EventDispatchers|AssignOnActorEndOverlap (Variables|Default|GetLeftPlatform) (delegate Custom|OnActorEndOverlap_Event_0))
      (EventDispatchers|AssignOnActorBeginOverlap (Variables|Default|GetRightPlatform) (delegate Custom|OnActorBeginOverlap_Event_1))
      (EventDispatchers|AssignOnActorEndOverlap (Variables|Default|GetRightPlatform) (delegate Custom|OnActorEndOverlap_Event_1)))))

(event EventTick
  (params (DeltaSeconds :type Float%20%28single-precision%29))
  (Utilities|FlowControl|Sequence
    (:then_0
      (for _array_element (Variables|Default|GetLeftOverlappingActors)
        (Physics|AddForce (Variables|Default|GetRightPhysicsActor) (* "0, 0,9.807000" (Physics|GetMass _array_element)) "None" true)))
    (:then_1
      (for _array_element_2 (Variables|Default|GetRightOverlappingActors)
        (Physics|AddForce (Variables|Default|GetLeftPhysicsActor) (* "0, 0,9.807000" (Physics|GetMass _array_element_2)) "None" true)))
    (:then_2
      (CallFunction|ClampZLocation (Variables|Default|GetLeftPhysicsActor))
      (CallFunction|ClampZLocation (Variables|Default|GetRightPhysicsActor)))))

(fn ConstructionScript)

(fn ClampZLocation
  (params (PhysicsActor :type Scene%20Component%20Object%20Reference))
  (bind _returnvalue (Transformation|GetWorldLocation PhysicsActor))
  (bind _distancetofloor (Variables|Default|GetDistanceToFloor))
  (bind _initialworldz (Variables|Default|GetInitialWorldZ))
  (Transformation|SetWorldLocation PhysicsActor (Math|Vector|MakeVector (.x _returnvalue) (.y _returnvalue) (Math|Float|Clamp(Float) (.z _returnvalue) (- _initialworldz _distancetofloor) (+ _initialworldz _distancetofloor))) false false))