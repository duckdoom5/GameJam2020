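; Game mode Blueprint that sets up a shared camera view and a second local player on BeginPlay.
; It points player 0's view at the last BP_Camera found in the level and creates the second player with its own controller.
; A one-shot timer calls SlamEgg, which is unfinished: it gathers BP_Player actors, averages their locations and casts the first, but uses none of the results.
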(event Custom|SlamEgg
  (bind _outactors (Actor|GetAllActorsOfClass "/Game/Blueprints/Player/BP_Player.BP_Player_C"))
  (Class|GameplayStatics|GetActorArrayAverageLocation _outactors)
  (Utilities|Casting|CastToBP_Player (Utilities|Array|Get(acopy) _outactors))
  (Utilities|Casting|CastToBP_Player (Utilities|Array|Get(acopy) _outactors)))

(event EventTick
  (params (DeltaSeconds :type Float%20%28single-precision%29)))

(event EventBeginPlay
  (Utilities|Time|SetTimerbyEvent (delegate Custom|SlamEgg) 1e+01)
  (Utilities|FlowControl|Sequence
    (:then_0
      (bind _outactors (Actor|GetAllActorsOfClass "/Game/Blueprints/BP_Camera.BP_Camera_C"))
      (Game|Player|SetViewTargetwithBlend (Game|GetPlayerController 0) (Utilities|Array|Get(acopy) _outactors (Utilities|Array|LastIndex _outactors)) 0.0 "VTBlend_Linear" 0.0 false)
      (Class|GameplayStatics|CreatePlayer 1))))

(fn ConstructionScript)