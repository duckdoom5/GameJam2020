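; BP_EggTimer is an egg timer that winds down visually and then shakes as if ringing.
; On BeginPlay it offsets the Top component's yaw in proportion to TimerSeconds and starts a looping countdown timer.
; Each tick unwinds the yaw and decrements TimerSeconds.
; At zero it pauses the countdown and starts a second looping timer that rocks Top's pitch back and forth indefinitely, with no sound.
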(event Custom|Countdown_Visuals
  (bind _top (Variables|Default|GetTop))
  ;[1 1 1] CountdownTimer
  (Transformation|SetWorldRotation _top (Math|Rotator|MakeRotator 0.0 0.0 (- (.yaw (Transformation|GetWorldRotation _top)) 0.045)) false false)
  (Variables|Default|SetTimerSeconds (- (Variables|Default|GetTimerSeconds) 0.01))
  (if (not (> (- (Variables|Default|GetTimerSeconds) 0.01) 0.0))
    (Utilities|Time|PauseTimerbyHandle (stale EventBeginPlay _returnvalue))
    (Utilities|Time|SetTimerbyEvent (delegate Custom|rINGrING) 0.15 true)))

(event Custom|rINGrING
  (bind _top (Variables|Default|GetTop))
  (bind _top_2 (Variables|Default|GetTop))
  (bind _returnvalue (Transformation|GetWorldRotation _top))
  ;[1 1 1] CompleteTimer
  (Transformation|SetWorldRotation _top_2 (Math|Rotator|MakeRotator 0.0 -2.0 (.yaw _returnvalue)) false false)
  (Utilities|FlowControl|Delay 0.05)
  (Transformation|SetWorldRotation _top_2 (Math|Rotator|MakeRotator 0.0 0.0 (.yaw _returnvalue)) false false)
  (Utilities|FlowControl|Delay 0.05)
  (Transformation|SetWorldRotation _top_2 (Math|Rotator|MakeRotator 0.0 2.0 (.yaw _returnvalue)) false false))

(event EventBeginPlay
  (bind _top (Variables|Default|GetTop))
  ;[1 1 1] SetStartingLocation
  (Transformation|SetWorldRotation _top (Math|Rotator|MakeRotator 0.0 0.0 (+ (.yaw (Transformation|GetWorldRotation _top)) (* (Variables|Default|GetTimerSeconds) 4.5))) false false)
  (bind _returnvalue (Utilities|Time|SetTimerbyEvent (delegate Custom|Countdown_Visuals) 0.01 true)))

(fn ConstructionScript)